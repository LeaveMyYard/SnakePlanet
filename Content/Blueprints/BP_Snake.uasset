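; BP_Snake is the player snake in a Snake-style game on a spherical planet, with steering enabled after an intro camera-arm timeline.
; Tick projects movement onto the planet surface using spherical coordinates; input rotates the heading around the surface normal.
; BP_Trail segments follow spaced samples from a rolling position history.
; Food adds segments and updates score and quadratic level thresholds; hitting trail beyond two name-excluded segments triggers death and pauses.
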(event OnComponentBeginOverlap(SnakeHead)
  (params (OverlappedComponent :type Primitive%20Component%20Object%20Reference) (OtherActor :type Actor%20Object%20Reference) (OtherComp :type Primitive%20Component%20Object%20Reference) (OtherBodyIndex :type Integer) (bFromSweep :type Boolean) (SweepResult :type Hit%20Result%20Structure%20%28by%20ref%29))
  (bind _returnvalue (Utilities|GetObjectName OtherActor))
  (if (Math|Boolean|ANDBoolean (Utilities|Enum|NotEqual(Enum) _returnvalue "BP_Trail_C_0") (Utilities|Enum|NotEqual(Enum) _returnvalue "BP_Trail_C_1") (Variables|Default|GetStarted) (== (Utilities|GetClass OtherActor) "/Game/Blueprints/BP_Trail.BP_Trail_C"))
    (CallFunction|EventDead)))

(event Custom|Event%20Food%20Eaten
  (bind _path (Variables|Default|GetPath))
  (Math|Integer|IncrementInt (Variables|Default|GetSize)
    (:%20%20
      (for _index (range 1 (Variables|Default|GetPointsPerBone))
        (Utilities|Array|Add (Variables|Default|GetPath) (Variables|Default|GetLook)))
      (bind _returnvalue (Game|SpawnActorfromClass "/Game/Blueprints/BP_Trail.BP_Trail_C" (Math|Transform|MakeTransform (Utilities|Array|Get(acopy) _path (- (Utilities|Array|Length _path) 1))) "Undefined" 0 0))
      (Utilities|Array|Add (Variables|Default|GetTrail) _returnvalue)
      (CallFunction|UpdateScore)
      (Audio|PlaySound2D "/Engine/VREditor/Sounds/UI/Selection_Changes.Selection_Changes" 1.0 1.0 0.0 0 0))))

(event Custom|Event%20Dead
  (Default|SetDead (.AsBP%20HUD (Utilities|Casting|CastToBP_HUD (HUD|GetHUD (Game|GetPlayerController 0)))))
  (Audio|PlaySound2D "/Engine/VREditor/Sounds/VR_close.VR_close" 1.0 1.0 0.0 0 0)
  (Game|SetGamePaused true))

(event Custom|Start
  (bind _newtrack_0 (Timeline|Timeline_0 PlayFromStart)
    (:Update
      (Variables|/Script/Engine.SpringArmComponent|SetTargetArmLength (Variables|Default|GetSpringArm) _newtrack_0))
    (:Finished
      (Variables|Default|SetStarted true)
      (Default|SpawnFood (Variables|Default|GetPlanet))
      (CallFunction|UpdateScore))))

(event EventBeginPlay
  (bind _planet (Variables|Default|GetPlanet))
  (bind _size (Variables|Default|GetSize))
  (bind _returnvalue (Transformation|GetActorLocation _planet))
  (bind (_x _y _z) (Math|Vector|BreakVector _returnvalue))
  (Variables|Default|SetLook (Math|Vector|Normalize (Variables|Default|GetLook)))
  (Transformation|SetActorLocation self (Math|Vector|MakeVector (+ _x (Default|GetPlanetRadius _planet)) _y _z) false false)
  (for _index (range 0 (* _size (Variables|Default|GetPointsPerBone)))
    (Utilities|Array|Add (Variables|Default|GetPath) (Variables|Default|GetLook)))
  (for _index_2 (range 1 _size)
    (bind _returnvalue_2 (Game|SpawnActorfromClass "/Game/Blueprints/BP_Trail.BP_Trail_C" (Transformation|GetActorTransform) "Undefined" 0 0))
    (Utilities|Array|Add (Variables|Default|GetTrail) _returnvalue_2)))

(event EventTick
  (params (DeltaSeconds :type Float%20%28single-precision%29))
  (bind _self self)
  (bind _planet (Variables|Default|GetPlanet))
  (bind _camera (Variables|Default|GetCamera))
  (bind _path (Variables|Default|GetPath))
  (bind _returnvalue (Transformation|GetActorLocation _self))
  (bind _returnvalue_2 (Transformation|GetWorldLocation _camera))
  (bind _returnvalue_3 (Transformation|GetActorLocation _planet))
  (bind _returnvalue_4 (Math|Rotator|FindLookatRotation _returnvalue_2 _returnvalue_3))
  (bind _output_get (Variables|Default|SetLastLocation _returnvalue))
  (bind _returnvalue_5 (Utilities|Array|Add (Variables|Default|GetPath) _output_get))
  (if (> _returnvalue_5 (* (+ (Variables|Default|GetSize) 1) (Variables|Default|GetPointsPerBone)))
    (Utilities|Array|RemoveIndex (Variables|Default|GetPath)))
  (Transformation|SetActorLocation self (+ (CallFunction|GetVectorbySpherical (Utilities|Struct|MakeSphereLocation (Default|GetPlanetRadius (Variables|Default|GetPlanet)) (.Phi (Utilities|Struct|BreakSphereLocation (CallFunction|GetSphericalbyVector (+ (- _returnvalue (Transformation|GetActorLocation (Variables|Default|GetPlanet))) (* (Variables|Default|GetLook) (* (Utilities|Time|GetWorldDeltaSeconds) (Variables|Default|GetSpeed))))))) (.Theta (Utilities|Struct|BreakSphereLocation (CallFunction|GetSphericalbyVector (+ (- _returnvalue (Transformation|GetActorLocation (Variables|Default|GetPlanet))) (* (Variables|Default|GetLook) (* (Utilities|Time|GetWorldDeltaSeconds) (Variables|Default|GetSpeed))))))))) (Transformation|GetActorLocation (Variables|Default|GetPlanet))) false false)
  (Variables|Default|SetLook (Math|Vector|Normalize (- (Transformation|GetActorLocation self) (Variables|Default|GetLastLocation))))
  (Transformation|SetRelativeRotation (Variables|Default|GetSnakeHead) _returnvalue_4 false false)
  (Transformation|SetRelativeRotation (Variables|Default|GetSpringArm) _returnvalue_4 false false)
  (for (_array_element _array_index) (Variables|Default|GetTrail)
    (Transformation|SetActorLocation _array_element (Utilities|Array|Get(acopy) _path (- (Utilities|Array|Length _path) (+ (* (+ _array_index 1) (Variables|Default|GetPointsPerBone)) 5))) false false)))

(event Input|AxisEvents|InputAxisMove
  (params (AxisValue :type Float%20%28single-precision%29))
  (if (Variables|Default|GetStarted)
    (Variables|Default|SetLook (Math|Vector|RotateVectorAroundAxis (Variables|Default|GetLook) (- 0.0 (* AxisValue (Utilities|Time|GetWorldDeltaSeconds) 1e+02)) (- (Transformation|GetActorLocation self) (Transformation|GetActorLocation (Variables|Default|GetPlanet)))))))

(fn ConstructionScript)

(fn UpdateScore
  (bind _current_level (Variables|Default|GetCurrent%20Level))
  (bind _size (Variables|Default|GetSize))
  (bind _returnvalue (- _size 5))
  (bind _returnvalue_2 (Math|Conversions|ToFloat(Integer) _current_level))
  (bind _returnvalue_3 (|(10+((5*k)*(k-1))) _returnvalue_2))
  (bind _returnvalue_4 (Math|Float|Truncate _returnvalue_3))
  (if (>= _returnvalue _returnvalue_4)
    (Math|Integer|IncrementInt (Variables|Default|GetCurrent%20Level)
      (:%20%20
        _)))
  (Default|SetScore (Variables|/Game/Widgets/BP_HUD.BP_HUD_C|GetScoreWidget (.AsBP%20HUD (Utilities|Casting|CastToBP_HUD (HUD|GetHUD (Game|GetPlayerController 0))))) _returnvalue _returnvalue_4 _current_level))