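; BP_Sun is a sun actor that spawns a single BP_Planet at a fixed offset along negative world X on BeginPlay and stores it as MainPlanet.
; An orbit routine rotates the planet's offset from the sun around the Z axis, scaled by delta seconds, and passes the result to the planet's MoveAt.
; That routine is disconnected from the empty Tick event, so it never runs.
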(event EventBeginPlay
  (bind _returnvalue (Game|SpawnActorfromClass "/Game/Blueprints/BP_Planet.BP_Planet_C" (Math|Transform|MakeTransform (Math|Vector|MakeVector -1.5e+03 0.0 0.0) "0, 0, 0" "1,1,1.000000") "Undefined" 0 0))
  (Variables|Default|SetMainPlanet _returnvalue))

(event EventTick
  (params (DeltaSeconds :type Float%20%28single-precision%29)))

(fn ConstructionScript)