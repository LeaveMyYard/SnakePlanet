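; BP_Moon is the spherical planet for a Snake game, serving as the surface on which food spawns.
; The construction script scales the sphere mesh from PlanetRadius, which is also exposed through a getter.
; SpawnFood converts random spherical angles into a point at that radius around the actor and stores the spawned food.
; MoveAt shifts the snake, food and moon together by the same local offset derived from a target location.
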(fn ConstructionScript
  (bind _planet_radius (Variables|Default|GetPlanet%20Radius))
  (bind _returnvalue (* _planet_radius 3.6))
  (bind _returnvalue_2 (/ _returnvalue 2e+02))
  (Transformation|SetWorldScale3D (Variables|Default|GetSphere) (Math|Vector|MakeVector _returnvalue_2 _returnvalue_2 _returnvalue_2)))

(fn GetPlanetRadius
  (return (Variables|Default|GetPlanet%20Radius)))

(fn SpawnFood
  (bind _returnvalue (Math|Trig|GetPI))
  (bind _returnvalue_2 (Game|SpawnActorfromClass "/Game/Blueprints/BP_Food.BP_Food_C" (Math|Transform|MakeTransform (+ (CallFunction|GetVectorbySpherical (Utilities|Struct|MakeSphereLocation (Variables|Default|GetPlanet%20Radius) (Math|Random|RandomFloatinRange 0.0 (* (Math|Trig|GetPI) 2.0)) (Math|Random|RandomFloatinRange (* _returnvalue -1.0) _returnvalue))) (Transformation|GetActorLocation))) "Undefined" 0 0))
  (Variables|Default|SetFood _returnvalue_2))

(fn Moveat
  (params (Location :type Vector))
  (bind _returnvalue (Transformation|GetActorLocation))
  (bind _returnvalue_2 (- Location _returnvalue))
  (Transformation|AddActorLocalOffset (Variables|Default|GetSnake) _returnvalue_2 false false)
  (Transformation|AddActorLocalOffset (Variables|Default|GetFood) _returnvalue_2 false false)
  (Transformation|AddActorLocalOffset self _returnvalue_2 false false))