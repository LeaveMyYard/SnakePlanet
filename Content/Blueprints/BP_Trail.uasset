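; BP_Trail is a trail actor for a snake game, with an overlap sphere meant to kill BP_Snake.
; On Sphere1 overlap it calls EventDead if the other actor is BP_Snake and its own overlapped component is named "SnakeHead".
; SpawnFood places BP_Food at random spherical angles around itself, but with zero radius; GetPlanetRadius also returns zero.
; MoveAt offsets the Snake reference and the trail toward a location, applying the trail's offset twice.
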(event OnComponentBeginOverlap(Sphere1)
  (params (OverlappedComponent :type Primitive%20Component%20Object%20Reference) (OtherActor :type Actor%20Object%20Reference) (OtherComp :type Primitive%20Component%20Object%20Reference) (OtherBodyIndex :type Integer) (bFromSweep :type Boolean) (SweepResult :type Hit%20Result%20Structure%20%28by%20ref%29))
  (bind _asbp_snake (Utilities|Casting|CastToBP_Snake OtherActor))
  (if (and (== (Utilities|GetClass OtherActor) "/Game/Blueprints/BP_Snake.BP_Snake_C") (Utilities|Enum|Equal(Enum) (Utilities|GetObjectName OverlappedComponent) "SnakeHead"))
    (Utilities|IsValid _asbp_snake
      (:Is%20Valid
        (Default|EventDead _asbp_snake)))))

(fn ConstructionScript)

(fn GetPlanetRadius
  (return 0.0))

(fn SpawnFood
  (bind _returnvalue (Math|Trig|GetPI))
  (Game|SpawnActorfromClass "/Game/Blueprints/BP_Food.BP_Food_C" (Math|Transform|MakeTransform (+ (CallFunction|GetVectorbySpherical (Utilities|Struct|MakeSphereLocation 0.0 (Math|Random|RandomFloatinRange 0.0 (* (Math|Trig|GetPI) 2.0)) (Math|Random|RandomFloatinRange (* _returnvalue -1.0) _returnvalue))) (Transformation|GetActorLocation))) "Undefined" 0 0))

(fn Moveat
  (params (Location :type Vector))
  (bind _returnvalue (Transformation|GetActorLocation))
  (bind _returnvalue_2 (- Location _returnvalue))
  (Transformation|AddActorLocalOffset (Variables|Default|GetSnake) _returnvalue_2 false false)
  (Transformation|AddActorLocalOffset _returnvalue_2 false false)
  (Transformation|AddActorLocalOffset self _returnvalue_2 false false))