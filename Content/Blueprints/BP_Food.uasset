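; BP_Food is the food pickup for a snake game set on a planet.
; On BeginPlay it caches the first BP_Planet found in the level.
; When a BP_Snake overlaps its sphere, it has the planet spawn new food, notifies the snake through EventFoodEaten, then destroys itself.
; A timeline for vertically offsetting the mesh exists but is never triggered.
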(event OnComponentBeginOverlap(Sphere)
  (params (OverlappedComponent :type Primitive%20Component%20Object%20Reference) (OtherActor :type Actor%20Object%20Reference) (OtherComp :type Primitive%20Component%20Object%20Reference) (OtherBodyIndex :type Integer) (bFromSweep :type Boolean) (SweepResult :type Hit%20Result%20Structure%20%28by%20ref%29))
  (bind _asbp_snake (Utilities|Casting|CastToBP_Snake OtherActor))
  (if (== (Utilities|GetClass OtherActor) "/Game/Blueprints/BP_Snake.BP_Snake_C")
    (Default|SpawnFood (Variables|Default|GetPlanet))
    (Utilities|IsValid _asbp_snake
      (:Is%20Valid
        (Default|EventFoodEaten _asbp_snake))
      (:Is%20Not%20Valid
        _))
    (Actor|DestroyActor)))

(event EventBeginPlay
  (bind _outactors (Actor|GetAllActorsOfClass "/Game/Blueprints/BP_Planet.BP_Planet_C"))
  (Variables|Default|SetPlanet (Utilities|Array|Get(acopy) _outactors)))

(fn ConstructionScript)