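; A Blueprint function library for spherical coordinate math using a SphereLocation struct of Radius, Theta and Phi.
; It converts between spherical locations and Cartesian vectors, using math expression nodes one way and Acos and Atan2 the other, with Theta measured from the Z axis.
; It also adds two locations component-wise without wrapping the angles, and formats a location as a readable string.
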(fn GetVectorbySpherical
  (params (Sphere%20Location :type Sphere%20Location%20Structure))
  (bind (_radius _phi _theta) (Utilities|Struct|BreakSphereLocation Sphere%20Location))
  (return (Math|Vector|MakeVector (|((r*(sin(t)))*(cos(p))) _radius _theta _phi) (|((r*(sin(t)))*(sin(p))) _radius _phi _theta) (|(r*(cos(t))) _radius _theta))))

(fn GetSphericalbyVector
  (params (Location :type Vector))
  (bind _returnvalue (Math|Vector|VectorLength Location))
  (bind (_x _y _z) (Math|Vector|BreakVector Location))
  (return (Utilities|Struct|MakeSphereLocation _returnvalue (Math|Trig|Atan2(Radians) _y _x) (Math|Trig|Acos(Degrees) (/ _z _returnvalue)))))

(fn AddSphericalCoordinates
  (params (Sphere%201 :type Sphere%20Location%20Structure) (Sphere%202 :type Sphere%20Location%20Structure))
  (bind (_radius _phi _theta) (Utilities|Struct|BreakSphereLocation Sphere%201))
  (bind (_radius_2 _phi_2 _theta_2) (Utilities|Struct|BreakSphereLocation Sphere%202))
  (return (Utilities|Struct|MakeSphereLocation (+ _radius _radius_2) (+ _phi _phi_2) (+ _theta _theta_2))))

(fn ToString
  (params (Sphere :type Sphere%20Location%20Structure))
  (bind (_radius _phi _theta) (Utilities|Struct|BreakSphereLocation Sphere))
  (return (Utilities|String|ToString(Text) (Utilities|Text|FormatText "Radius: {a}, Phi: {b}, Theta: {c}" _radius _phi _theta))))